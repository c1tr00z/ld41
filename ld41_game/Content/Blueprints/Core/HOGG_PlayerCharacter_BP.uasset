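; Player character Blueprint that handles look and movement axis input.
; Vertical look pitches the Camera component directly, applying input only while pitch stays strictly within 90 degrees of level, while horizontal look adds yaw to the controller's control rotation.
; Movement feeds the Camera's forward and right vectors into AddMovementInput, so the forward direction passed in includes camera pitch.
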(event `InputAxis|LookUp`
  (params (AxisValue :type "Float (single-precision)"))
  (`self.LookUp` AxisValue))

(event `InputAxis|LookRight`
  (params (AxisValue :type "Float (single-precision)"))
  (`self.LookRight` AxisValue))

(event `InputAxis|MoveRight`
  (params (AxisValue :type "Float (single-precision)"))
  (`self.MoveRight` AxisValue))

(event `InputAxis|MoveUp`
  (params (AxisValue :type "Float (single-precision)"))
  (`self.MoveForward` AxisValue))

(fn `LookRight`
  (params (Value :type "Float (double-precision)"))
  (bind _returnvalue (`self.GetController`))
  (bind (_returnvalue_roll _returnvalue_pitch _returnvalue_yaw) (`KismetMathLibrary.BreakRotator` (`Controller.GetControlRotation` _returnvalue)))
  (`Controller.SetControlRotation` _returnvalue (`KismetMathLibrary.MakeRotator` _returnvalue_roll _returnvalue_pitch (+ _returnvalue_yaw Value))))

(fn `LookUp`
  (params (Value :type "Float (double-precision)"))
  (bind _camera (`self.Camera`))
  (bind (_relativerotation_roll _relativerotation_pitch) (`KismetMathLibrary.BreakRotator` (`SceneComponent.RelativeRotation` _camera)))
  (bind _returnvalue (+ _relativerotation_pitch Value))
  (if (and (< _returnvalue 90.0) (> _returnvalue -90.0))
    (`SceneComponent.K2_AddRelativeRotation` _camera (`KismetMathLibrary.MakeRotator` 0.0 Value) false false)))

(fn `MoveForward`
  (params (Value :type "Float (double-precision)"))
  (`self.AddMovementInput` (`SceneComponent.GetForwardVector` (`self.Camera`)) Value))

(fn `MoveRight`
  (params (Value :type "Float (double-precision)"))
  (`self.AddMovementInput` (`SceneComponent.GetRightVector` (`self.Camera`)) Value))

(fn `UserConstructionScript`)